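; Player spaceship for an asteroid shooter, steered with physics torque for rotation and force along its right vector for thrust.
; The shoot input plays a laser sound and spawns a bullet at a scene component's transform.
; Overlapping an asteroid destroys it and calls HealthF, which decrements health and hides one of two extra ship components.
; At zero health the ship plays a tone, destroys itself and opens the main menu level.
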(event `self.spaceshipColligion.OnComponentBeginOverlap`
  (params (OverlappedComponent :type "PrimitiveComponent Object Reference") (OtherActor :type "Actor Object Reference") (OtherComp :type "PrimitiveComponent Object Reference") (OtherBodyIndex :type Integer) (bFromSweep :type Boolean) (SweepResult :type "HitResult Structure (by ref)"))
  (bind _asastroid_base_bp (cast `/Game/astroidBase_BP` OtherActor))
  (`GameplayStatics.PlaySound2D` "/Game/Assets/StaticMashes/Sound/explo.explo" 1.0 1.0 0.0 null null)
  (`self.K2_DestroyActor` _asastroid_base_bp)
  (`self.HealthF`))

(event `InputAxis|rotation`
  (params (AxisValue :type "Float (single-precision)"))
  (`PrimitiveComponent.AddTorqueInDegrees` (`self.spaceship`) (`KismetMathLibrary.MakeVector` 0.0 0.0 (* AxisValue (`self.RotationMulti`))) "None" true))

(event `InputAxis|Move`
  (params (AxisValue :type "Float (single-precision)"))
  (bind _spaceship (`self.spaceship`))
  (`PrimitiveComponent.AddForce` _spaceship (* (`SceneComponent.GetRightVector` _spaceship) (`KismetMathLibrary.FTrunc` (* AxisValue (`self.MoveMulti`)))) "None" true))

(event `InputAction|shoot`
  (params (Key :type "Key Structure"))
  (:`Pressed`
    (`GameplayStatics.PlaySound2D` "/Game/Assets/StaticMashes/Sound/laserShoot.laserShoot" 1.0 1.0 0.0 null null)
    (`|SpawnActorFromClass` "/Game/Bullet_BP.Bullet_BP_C" (`SceneComponent.K2_GetComponentToWorld` (`self.Scene`)) "AlwaysSpawn" "OverrideRootScale" null null)))

(fn `HealthF`
  (bind _output_get (set `self.health` (- (`self.health`) 1)))
  (switch `int` _output_get
    (:`0`
      (`GameplayStatics.PlaySound2D` "/Game/Assets/StaticMashes/Sound/tone.tone" 1.0 1.0 0.0 null null)
      (`self.K2_DestroyActor`)
      (`GameplayStatics.OpenLevel` "MainManu_Level"))
    (:`1`
      (`SceneComponent.SetVisibility` (`self.spaceship2`) false false))
    (:`2`
      (`SceneComponent.SetVisibility` (`self.spaceship3`) false false))))

(fn `UserConstructionScript`)