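; Base asteroid actor that drifts across the XY plane and splits when its bullet-touch function is called.
; BeginPlay picks a random, unnormalized XY direction, and Tick offsets the static mesh by it times Speed, without delta-time scaling or sweep.
; BulletTouch spawns two AstroidBase_BP_2_O_Child actors at the mesh's transform, plays an explosion sound and destroys the asteroid.
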(event `self.ReceiveBeginPlay`
  (set `self.Random ` (`KismetMathLibrary.MakeVector` (`KismetMathLibrary.RandomFloatInRange` -1.0 1.0) (`KismetMathLibrary.RandomFloatInRange` -1.0 1.0))))

(event `self.ReceiveTick`
  (params (DeltaSeconds :type "Float (single-precision)"))
  (`SceneComponent.K2_AddWorldOffset` (`self.StaticMesh`) (* (`self.Random `) (`self.speed`)) false false))

(fn `bullet_touch`
  (`|SpawnActorFromClass` "/Game/astroidBase_BP_2_O_Child.astroidBase_BP_2_O_Child_C" (`SceneComponent.K2_GetComponentToWorld` (`self.StaticMesh`)) "AdjustIfPossibleButAlwaysSpawn" "OverrideRootScale" null null)
  (`|SpawnActorFromClass` "/Game/astroidBase_BP_2_O_Child.astroidBase_BP_2_O_Child_C" (`SceneComponent.K2_GetComponentToWorld` (`self.StaticMesh`)) "AdjustIfPossibleButAlwaysSpawn" "OverrideRootScale" null null)
  (`GameplayStatics.PlaySound2D` "/Game/Assets/StaticMashes/Sound/explosion.explosion" 1.0 1.0 0.0 null null)
  (`self.K2_DestroyActor`))

(fn `UserConstructionScript`)